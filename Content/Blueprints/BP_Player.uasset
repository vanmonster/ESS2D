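; BP_Player is a 2D Paper2D player character that moves sideways, up and down on the X-Z plane.
; Enhanced Input actions from IMC_ESS2D add movement, and side input flips the controller yaw to face the travel direction.
; Every Tick, the last input vector selects the idle, side, up or down flipbook, with vertical overriding side.
; BeginPlay also creates the WB_UI widget and starts a looping timer that feeds it a seconds counter.
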(event `self.ReceiveBeginPlay`
  (`self.Add_IMC`)
  ;[1 1 1] Виджет времени
  (bind _returnvalue (`|CreateWidget` "/Game/Blueprints/WB_UI.WB_UI_C"))
  (bind _output_get (set `self.Time` _returnvalue))
  (`UserWidget.AddToViewport` _output_get 0)
  (`KismetSystemLibrary.K2_SetTimerDelegate` (delegate `UpdateTime`) 1.0 true))

(event `UpdateTime`
  ;[1 1 1] Виджет времени
  (bind _result (`/Engine/EditorBlueprintResources/StandardMacros.IncrementInt` (`self.Time_integer`))
    (:`  `
      (`/Game/Blueprints/WB_UI.UpdateTime` (`self.Time`) _result))))

(event `self.ReceiveTick`
  (params (DeltaSeconds :type "Float (single-precision)"))
  (`self.UpdateAnimationSide`)
  (`self.UpdateAnimationUp`)
  (`self.UpdateAnimationDown`)
  (`self.UpdateAnimationIdle`))

(event `EnhancedInput|/Game/Input/Actions/IA_Side`
  (params (ActionValue :type "Float (double-precision)") (ElapsedSeconds :type "Float (double-precision)") (TriggeredSeconds :type "Float (double-precision)") (InputAction :type "InputAction Object Reference" :default "/Game/Input/Actions/IA_Side.IA_Side"))
  ;[1 1 1] Управление игроком.
  (:`Triggered`
    (`self.AddMovementInput` (1.0 0.0 0.0) ActionValue)
    (`Controller.SetControlRotation` (`self.GetController`) (select `bool` (> ActionValue 0.0) :`false` (`KismetMathLibrary.MakeRotator` 0.0 0.0 180.0) :`true` (`KismetMathLibrary.MakeRotator` 0.0)))))

(event `EnhancedInput|/Game/Input/Actions/IA_Up`
  (params (ActionValue :type "Float (double-precision)") (ElapsedSeconds :type "Float (double-precision)") (TriggeredSeconds :type "Float (double-precision)") (InputAction :type "InputAction Object Reference" :default "/Game/Input/Actions/IA_Up.IA_Up"))
  ;[1 1 1] Управление игроком.
  (:`Triggered`
    (`self.AddMovementInput` (0.0 0.0 1.0) ActionValue)))

(event `EnhancedInput|/Game/Input/Actions/IA_Down`
  (params (ActionValue :type "Float (double-precision)") (ElapsedSeconds :type "Float (double-precision)") (TriggeredSeconds :type "Float (double-precision)") (InputAction :type "InputAction Object Reference" :default "/Game/Input/Actions/IA_Down.IA_Down"))
  ;[1 1 1] Управление игроком.
  (:`Triggered`
    (`self.AddMovementInput` (0.0 0.0 -1.0) ActionValue)))

(fn `Add_IMC`
  ;[1 1 1] Добавление контроллера игрока.
  (bind _asplayer_controller (cast `PlayerController` (`self.GetController`)))
  (`EnhancedInputSubsystemInterface.AddMappingContext` (pcsubsystem `EnhancedInputLocalPlayerSubsystem` _asplayer_controller) "/Game/Input/IMC_ESS2D.IMC_ESS2D" 0 (struct)))

(fn `UpdateAnimationDown`
  (bind (_returnvalue_x _returnvalue_y _returnvalue_z) (`KismetMathLibrary.BreakVector` (`PawnMovementComponent.GetLastInputVector` (`self.CharacterMovement`))))
  (if (< _returnvalue_z 0.0)
    (`PaperFlipbookComponent.SetFlipbook` (`self.Sprite`) "/Game/Assets/Player/Flipbooks/Down.Down")))

(fn `UpdateAnimationIdle`
  (if (== (`KismetMathLibrary.VSize` (`PawnMovementComponent.GetLastInputVector` (`self.CharacterMovement`))) 0.0)
    (`PaperFlipbookComponent.SetFlipbook` (`self.Sprite`) "/Game/Assets/Player/Flipbooks/Idle.Idle")))

(fn `UpdateAnimationSide`
  (bind _returnvalue_x (`KismetMathLibrary.BreakVector` (`PawnMovementComponent.GetLastInputVector` (`self.CharacterMovement`))))
  (if (!= _returnvalue_x 0.0)
    (`PaperFlipbookComponent.SetFlipbook` (`self.Sprite`) "/Game/Assets/Player/Flipbooks/Side.Side")))

(fn `UpdateAnimationUp`
  (bind (_returnvalue_x _returnvalue_y _returnvalue_z) (`KismetMathLibrary.BreakVector` (`PawnMovementComponent.GetLastInputVector` (`self.CharacterMovement`))))
  (if (> _returnvalue_z 0.0)
    (`PaperFlipbookComponent.SetFlipbook` (`self.Sprite`) "/Game/Assets/Player/Flipbooks/Up.Up")))

(fn `UserConstructionScript`)